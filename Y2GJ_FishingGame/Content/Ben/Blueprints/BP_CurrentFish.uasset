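; BP_CurrentFish is an actor that displays the current fish, recording each one made and later showing them again to be eaten.
; MakeFish picks a random mesh, stores it, raises the fish count and tells BP_CaughtFish to change its mesh.
; ShowFish resets position and removes the mesh at the count index from the list to display it.
; EatFish shows bones, waits, then shows the next fish or starts the player's ShopPhase once the count runs out.
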(event `self.ReceiveBeginPlay`
  (set `self.StartPos` (`self.K2_GetActorLocation`)))

(event `MakeFish`
  (bind _mesh (`self.Mesh`))
  (set `self.PointValue` 5)
  (`StaticMeshComponent.SetStaticMesh` (`self.Mesh`) (`KismetArrayLibrary.Array_Random` (`self.FishMeshPossible`)))
  (`KismetArrayLibrary.Array_Add` (`self.FishMeshes`) (`StaticMeshComponent.StaticMesh` _mesh))
  (`KismetSystemLibrary.PrintString` (`KismetSystemLibrary.GetDisplayName` _mesh))
  (bind _result (`/Engine/EditorBlueprintResources/StandardMacros.IncrementInt` (`self.FishTotal`))
    (:`  `
      (set `self.FishTotal` _result)
      (bind _returnvalue (`GameplayStatics.GetActorOfClass` "/Game/Ben/Blueprints/BP_CaughtFish.BP_CaughtFish_C"))
      (`/Game/Ben/Blueprints/BP_CaughtFish.ChangeMyMesh` _returnvalue))))

(event `ResetPos`
  (`self.K2_SetActorLocation` (`self.StartPos`)))

(event `ShowFish`
  (bind _fishmeshes (`self.FishMeshes`))
  (bind _fishtotal (`self.FishTotal`))
  (`self.ResetPos`)
  (`StaticMeshComponent.SetStaticMesh` (`self.Mesh`) (`|GetArrayItem` _fishmeshes _fishtotal))
  (`KismetArrayLibrary.Array_Remove` _fishmeshes _fishtotal))

(event `EatFish`
  (`StaticMeshComponent.SetStaticMesh` (`self.Mesh`) "/Game/Fab/Stylized_Dark_Green_Pet_Bowl_and_Bone_Toy_Free_low-poly_3D_model/BoneToy_low.BoneToy_low")
  (`KismetSystemLibrary.Delay` 1.0)
  (bind _result (`/Engine/EditorBlueprintResources/StandardMacros.DecrementInt` (`self.FishTotal`))
    (:`  `
      (set `self.FishTotal` _result)
      (if (== (`self.FishTotal`) -1)
        (bind _returnvalue (`GameplayStatics.GetActorOfClass` "/Game/FirstPerson/Blueprints/BP_FirstPersonCharacter.BP_FirstPersonCharacter_C"))
        (`/Game/FirstPerson/Blueprints/BP_FirstPersonCharacter.ShopPhase` _returnvalue)
        (else
          (`self.ShowFish`))))))

(fn `UserConstructionScript`)