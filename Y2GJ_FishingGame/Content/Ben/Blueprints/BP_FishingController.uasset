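; Fishing controller actor that runs the cast, bite, hook and catch/fail flow for the player's fishing.
; Cast plays the FishGetter timeline from a CatchRate-based position; its finish opens a bite window timed by the CatchWindow timeline.
; Hooking within that window starts the character's minigame.
; Catch and Fail reset state, disable BP_PhysicsBar and notify the character, with Catch also calling MakeFish on BP_CurrentFish.
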(event `StartFishing`)

(event `Cast`
  (bind _returnvalue (`GameplayStatics.GetActorOfClass` "/Game/FirstPerson/Blueprints/BP_FirstPersonCharacter.BP_FirstPersonCharacter_C"))
  (set `/Game/FirstPerson/Blueprints/BP_FirstPersonCharacter.IsLineCast` true _returnvalue)
  (`|ExecutionSequence`
    (:`then_0`
      (`Timeline|FishGetter` :`NewTime` (+ (`KismetMathLibrary.RandomFloatInRange` 0.0 0.0) (`self.CatchRate`)) :!via `SetNewTime` :!label _label
        (:`Finished`
          (`KismetSystemLibrary.PrintString` "FISH!")
          (set `self.CanCatch` true)
          (`Timeline|CatchWindow` :!via `PlayFromStart`
            (:`Finished`
              (set `self.CanCatch` false))))))
    (:`then_1`
      (goto _label))))

(event `StopFish`
  (goto _label :!via `Stop`))

(event `Hook`
  (if (`self.CanCatch`)
    (`KismetSystemLibrary.PrintString` "SUCCESS")
    (set `self.InMinigame` true)
    (bind _returnvalue (`GameplayStatics.GetActorOfClass` "/Game/FirstPerson/Blueprints/BP_FirstPersonCharacter.BP_FirstPersonCharacter_C"))
    (`/Game/FirstPerson/Blueprints/BP_FirstPersonCharacter.ActivateMinigame` _returnvalue)
    (set `/Game/FirstPerson/Blueprints/BP_FirstPersonCharacter.IsLineCast` true _returnvalue)
    (`self.StopFish`)
    (else
      (`KismetSystemLibrary.PrintString` "FAILED")
      (`self.StopFish`)
      (bind _returnvalue_2 (`GameplayStatics.GetActorOfClass` "/Game/FirstPerson/Blueprints/BP_FirstPersonCharacter.BP_FirstPersonCharacter_C"))
      (set `/Game/FirstPerson/Blueprints/BP_FirstPersonCharacter.IsLineCast` false _returnvalue_2))))

(event `Catch`
  (bind _returnvalue (`GameplayStatics.GetActorOfClass` "/Game/FirstPerson/Blueprints/BP_FirstPersonCharacter.BP_FirstPersonCharacter_C"))
  (set `/Game/FirstPerson/Blueprints/BP_FirstPersonCharacter.IsLineCast` false _returnvalue)
  (set `self.InMinigame` false)
  (bind _returnvalue_2 (`GameplayStatics.GetActorOfClass` "/Game/Ben/Blueprints/BP_PhysicsBar.BP_PhysicsBar_C"))
  (`/Game/Ben/Blueprints/BP_PhysicsBar.Disable` _returnvalue_2)
  (bind _returnvalue_3 (`GameplayStatics.GetActorOfClass` "/Game/Ben/Blueprints/BP_CurrentFish.BP_CurrentFish_C"))
  (`/Game/Ben/Blueprints/BP_CurrentFish.MakeFish` _returnvalue_3)
  (bind _returnvalue_4 (`GameplayStatics.GetActorOfClass` "/Game/FirstPerson/Blueprints/BP_FirstPersonCharacter.BP_FirstPersonCharacter_C"))
  (`/Game/FirstPerson/Blueprints/BP_FirstPersonCharacter.CheckFinished` _returnvalue_4))

(event `Fail`
  (bind _returnvalue (`GameplayStatics.GetActorOfClass` "/Game/FirstPerson/Blueprints/BP_FirstPersonCharacter.BP_FirstPersonCharacter_C"))
  (set `/Game/FirstPerson/Blueprints/BP_FirstPersonCharacter.IsLineCast` false _returnvalue)
  (set `self.InMinigame` false)
  (bind _returnvalue_2 (`GameplayStatics.GetActorOfClass` "/Game/Ben/Blueprints/BP_PhysicsBar.BP_PhysicsBar_C"))
  (`/Game/Ben/Blueprints/BP_PhysicsBar.Disable` _returnvalue_2)
  (bind _returnvalue_3 (`GameplayStatics.GetActorOfClass` "/Game/FirstPerson/Blueprints/BP_FirstPersonCharacter.BP_FirstPersonCharacter_C"))
  (`/Game/FirstPerson/Blueprints/BP_FirstPersonCharacter.CheckFinished` _returnvalue_3))

(fn `UserConstructionScript`)