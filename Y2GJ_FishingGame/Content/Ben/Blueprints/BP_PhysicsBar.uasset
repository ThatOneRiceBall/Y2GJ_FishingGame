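; Fishing minigame bar actor that decides whether BP_FishingController registers a catch or a fail.
; MoveBarUp pushes a physics Cube upward while the RandomMove timeline moves Fishy vertically.
; Overlap opens a Tick-driven gate that raises Progress, while losing overlap closes it and starts a self-restarting LoopingFall timeline that drains Progress.
; Enable resets position and progress and creates the BP_FishingBar widget, which Disable hides.
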(event `self.ReceiveBeginPlay`
  (bind _fishy (`self.Fishy`))
  (bind (_relativelocation_x _relativelocation_y) (`KismetMathLibrary.BreakVector` (`SceneComponent.RelativeLocation` _fishy)))
  (set `self.DefaultFloor` (`self.K2_GetActorLocation`))
  (bind (_direction _time) (`Timeline|RandomMove`)
    (:`Update`
      (`SceneComponent.K2_SetRelativeLocation` _fishy (`KismetMathLibrary.MakeVector` _relativelocation_x _relativelocation_y _time) false false))))

(event `StopFall`
  (`Timeline|LoopingFall` :!via `Stop` :!label _label
    (:`Finished`
      (bind _output_get (set `self.Progress` (- (`self.Progress`) 0.005)))
      (if (<= _output_get 0.0)
        (`self.Disable`)
        (bind _returnvalue (`GameplayStatics.GetActorOfClass` "/Game/Ben/Blueprints/BP_FishingController.BP_FishingController_C"))
        (`/Game/Ben/Blueprints/BP_FishingController.Fail` _returnvalue)
        (else
          (goto _label :!via `PlayFromStart`))))))

(event `self.Fishy.OnComponentEndOverlap`
  (params (OverlappedComponent :type "PrimitiveComponent Object Reference") (OtherActor :type "Actor Object Reference") (OtherComp :type "PrimitiveComponent Object Reference") (OtherBodyIndex :type Integer))
  (`|ExecutionSequence`
    (:`then_0`
      (goto _label))
    (:`then_1`
      (goto _label_2 :!via `Close`))))

(event `self.ReceiveTick`
  (params (DeltaSeconds :type "Float (single-precision)"))
  (`/Engine/EditorBlueprintResources/StandardMacros.Gate` true :!label _label_2
    (:`Exit`
      (bind _output_get (set `self.Progress` (+ (`self.Progress`) 0.005)))
      (if (>= _output_get 1.0)
        (`/Engine/EditorBlueprintResources/StandardMacros.DoOnce` false :!label _label_3
          (:`Completed`
            (bind _returnvalue (`GameplayStatics.GetActorOfClass` "/Game/Ben/Blueprints/BP_FishingController.BP_FishingController_C"))
            (`/Game/Ben/Blueprints/BP_FishingController.Catch` _returnvalue)))))))

(event `self.Fishy.OnComponentBeginOverlap`
  (params (OverlappedComponent :type "PrimitiveComponent Object Reference") (OtherActor :type "Actor Object Reference") (OtherComp :type "PrimitiveComponent Object Reference") (OtherBodyIndex :type Integer) (bFromSweep :type Boolean) (SweepResult :type "HitResult Structure (by ref)"))
  (if (== OtherComp (`self.Cube`))
    (`|ExecutionSequence`
      (:`then_0`
        (goto _label_2 :!via `Open`))
      (:`then_1`
        (goto _label :!via `Stop`)))))

(event `Enable`
  (`/Engine/EditorBlueprintResources/StandardMacros.DoOnce` false :!label _label_4
    (:`Completed`
      (set `self.Active` true)
      (set `self.Progress` 0.5)
      (`self.K2_SetActorLocation` (`self.DefaultFloor`))
      (bind _returnvalue (`|CreateWidget` "/Game/Ben/UI/BP_FishingBar.BP_FishingBar_C"))
      (bind _output_get (set `self.UI` _returnvalue))
      (`UserWidget.AddToViewport` _output_get 0)
      (goto _label_3 :!via `Reset`))))

(event `Disable`
  (`self.StopFall`)
  (`Widget.SetVisibility` (`self.UI`) "Hidden")
  (set `self.Active` false)
  (goto _label_4 :!via `Reset`))

(event `MoveBarUp`
  (`PrimitiveComponent.AddForce` (`self.Cube`) (0.0 0.0 10000.0) "None" false))

(fn `UserConstructionScript`)