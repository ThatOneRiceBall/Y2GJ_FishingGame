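; BP_CaughtFish is an actor that briefly displays the fish the player has caught.
; Its ChangeMyMesh event adds the BP_FishUI and BP_CoinUp widgets to the viewport, then copies the static mesh from the BP_CurrentFish actor in the level.
; After a short delay it clears the mesh, while widget removal is not handled here.
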(event `ChangeMyMesh`
  (bind _returnvalue (`|CreateWidget` "/Game/Ben/UI/BP_FishUI.BP_FishUI_C"))
  (`UserWidget.AddToViewport` _returnvalue 0)
  (bind _returnvalue_2 (`|CreateWidget` "/Game/Ben/UI/BP_CoinUp.BP_CoinUp_C"))
  (`UserWidget.AddToViewport` _returnvalue_2 0)
  (bind _returnvalue_3 (`GameplayStatics.GetActorOfClass` "/Game/Ben/Blueprints/BP_CurrentFish.BP_CurrentFish_C"))
  (`StaticMeshComponent.SetStaticMesh` (`self.Mesh`) (`StaticMeshComponent.StaticMesh` (`/Game/Ben/Blueprints/BP_CurrentFish.Mesh` _returnvalue_3)))
  (`KismetSystemLibrary.Delay` 2.0)
  (`StaticMeshComponent.SetStaticMesh` (`self.Mesh`) null))

(fn `UserConstructionScript`)