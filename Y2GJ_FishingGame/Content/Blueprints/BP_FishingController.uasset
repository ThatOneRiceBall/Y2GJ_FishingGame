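; Fishing minigame controller that handles casting, timed bites and hook attempts, awarding points to the first-person character.
; Cast offsets the FishGetter timeline's start time by a random amount plus CatchRate; its completion opens a catch window timed by the CatchWindow timeline.
; Hook adds FishPoints to Score inside that window, otherwise stops the fish timer.
; StartFishing is empty, and the score Threshold branch only fetches the character.
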(event `StartFishing`)

(event `Cast`
  (`|ExecutionSequence`
    (:`then_0`
      (`Timeline|FishGetter` :`NewTime` (+ (`KismetMathLibrary.RandomFloatInRange` 0.0 4.0) (`self.CatchRate`)) :!via `SetNewTime` :!label _label
        (:`Finished`
          (`KismetSystemLibrary.PrintString` "FISH!")
          (set `self.CanCatch` true)
          (`Timeline|CatchWindow` :!via `PlayFromStart`
            (:`Finished`
              (set `self.CanCatch` false))))))
    (:`then_1`
      (goto _label))))

(event `StopFish`
  (goto _label :!via `Stop`))

(event `Hook`
  (if (`self.CanCatch`)
    (`KismetSystemLibrary.PrintString` "SUCCESS")
    (bind _returnvalue (`GameplayStatics.GetActorOfClass` "/Game/FirstPerson/Blueprints/BP_FirstPersonCharacter.BP_FirstPersonCharacter_C"))
    (bind _output_get (set `/Game/FirstPerson/Blueprints/BP_FirstPersonCharacter.Score` (+ (`/Game/FirstPerson/Blueprints/BP_FirstPersonCharacter.Score` _returnvalue) (`self.FishPoints`)) _returnvalue))
    (if (>= _output_get (`self.Threshold`))
      (`GameplayStatics.GetActorOfClass` "/Game/FirstPerson/Blueprints/BP_FirstPersonCharacter.BP_FirstPersonCharacter_C"))
    (else
      (`KismetSystemLibrary.PrintString` "FAILED")
      (`self.StopFish`))))

(fn `UserConstructionScript`)